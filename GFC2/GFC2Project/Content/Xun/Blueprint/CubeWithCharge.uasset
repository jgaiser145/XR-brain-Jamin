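; CubeWithCharge is a cube actor holding a boolean charge, with a function to compare it against another cube's charge, apparently an unfinished prototype.
; Each Tick, CubeTouch takes the first CubeWithCharge overlapping its sphere collision and clears that cube's TheOtherCube reference.
; Motion-controller touch detection through box collision, the charge check and lerped movement exist only as unconnected debug or draft logic that never runs.
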(event Custom|HandTouch
  (bind _outactors (Actor|GetAllActorsOfClass "/MixedRealityFramework/Calibration/VRTemplate/Blueprints/BP_MotionController.BP_MotionController_C"))
  (if (Collision|IsOverlappingActor (Variables|Default|GetBoxCollision) (Utilities|Array|Get(acopy) _outactors) :!class /Script/Engine.PrimitiveComponent)
    (Development|PrintString "Hello")))

(event Custom|CubeTouch
  (Utilities|IsValid self
    (:Is%20Valid
      (bind _ascube_with_charge (Utilities|Casting|CastToCubeWithCharge (Utilities|Array|Get(acopy) (Collision|GetOverlappingActors (Variables|Default|GetSphereCollision) "CubeWithCharge_C" :!class /Script/Engine.PrimitiveComponent))))
      (Variables|CubeWithCharge_C|SettheOtherCube _ascube_with_charge 0))))

(event EventBeginPlay)

(event Collision|EventActorBeginOverlap
  (params (OtherActor :type Actor%20Object%20Reference)))

(event EventTick
  (params (DeltaSeconds :type Float%20%28single-precision%29))
  (Utilities|FlowControl|Sequence
    (:then_1
      (CallFunction|CubeTouch))))

(fn ConstructionScript)

(fn GetMyCharge
  (return (Variables|Default|GetChargeBool)))

(fn SetMyCharge
  (params (SetMyCharge :type Boolean))
  (Variables|Default|SetChargeBool SetMyCharge))

(fn IsChargeSame
  (params (OtherCubeCharge :type Cube%20with%20Charge%20Object%20Reference))
  (bind _mychargebool (CallFunction|GetMyCharge))
  (bind _mychargebool_2 (CallFunction|GetMyCharge OtherCubeCharge))
  (return (Math|Boolean|Equal(Boolean) _mychargebool _mychargebool_2)))