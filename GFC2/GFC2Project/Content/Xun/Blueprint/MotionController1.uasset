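; MotionController1 is a pointer actor, apparently for a VR motion controller, that detects aimed-at objects tagged CubeWithCharge for moving.
; Each tick it draws a debug ray from ArrowDirection and line-traces WorldDynamic objects along it, ignoring all GridSpace actors.
; A tagged hit sets the VRCam pawn's OkToMove and ActorHitted.
; An untagged hit clears OkToMove, while no hit leaves the previous state intact.
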(event EventBeginPlay
  (|CallParentFunction) ; This node is disabled and will not be called.\nDrag off pins to build functionality.
)

(event Collision|EventActorBeginOverlap
  (params (OtherActor :type Actor%20Object%20Reference)))

(event EventTick
  (params (DeltaSeconds :type Float%20%28single-precision%29))
  (bind _returnvalue (Game|Player|GetPlayerPawn 0))
  (bind _arrowdirection (Variables|Default|GetArrowDirection))
  (bind _returnvalue_2 (Transformation|GetWorldLocation _arrowdirection))
  (bind _returnvalue_3 (Math|Vector|GetForwardVector _arrowdirection))
  (bind _returnvalue_4 (* _returnvalue_3 2e+04))
  (bind _returnvalue_5 (+ _returnvalue_2 _returnvalue_4))
  (Rendering|Debug|DrawDebugLine _returnvalue_2 _returnvalue_5 "(R=0.742709,G=0.126044,B=0.410306,A=1.000000)" 0.0 1.0)
  (bind _outactors (Actor|GetAllActorsOfClass "/Game/Peter/GridSpace.GridSpace_C"))
  (bind _outhit (Collision|LineTraceForObjects _returnvalue_2 _returnvalue_5 (Utilities|Array|MakeArray "ObjectTypeQuery2") false _outactors "None"))
  (bind _output_get (Variables|Default|SetactorHitted (.HitActor (Collision|BreakHitResult _outhit))))
  (Utilities|IsValid _output_get
    (:Is%20Valid
      (if (Actor|ActorHasTag _output_get "CubeWithCharge")
        (Variables|Default|SetOkToMove true)
        (bind _asvrcam (Utilities|Casting|CastToVRCam _returnvalue))
        (Default|SetOktoMove _asvrcam true)
        (Default|SetActorHitted _asvrcam (Variables|Default|GetactorHitted))
        (else
          (Variables|Default|SetOkToMove false)
          (bind _asvrcam_2 (Utilities|Casting|CastToVRCam _returnvalue))
          (Default|SetOktoMove _asvrcam_2 false))))))

(fn ConstructionScript
  (|CallParentFunction))