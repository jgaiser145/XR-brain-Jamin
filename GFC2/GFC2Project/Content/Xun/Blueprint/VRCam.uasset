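; VRCam is a VR player pawn that provides two tracked hands and axis-driven movement.
; On BeginPlay it sets a floor tracking origin, then spawns two BP_MotionController actors as left and right hands, attached to VRCamRoot.
; The forward and right input axes add movement along the control rotation's yaw only, ignoring pitch and roll.
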(event EventBeginPlay
  (bind _returnvalue (Math|Transform|MakeTransform "0, 0, 0"))
  (bind _self self)
  (bind _vrcamroot (Variables|Default|GetVRCamRoot))
  (Class|HeadMountedDisplayFunctionLibrary|SetTrackingOrigin "Floor")
  ;[1 1 1] Setting up hand
  (Utilities|FlowControl|Sequence
    (:then_0
      (bind _returnvalue_2 (Game|SpawnActorfromClass "/MixedRealityFramework/Calibration/VRTemplate/Blueprints/BP_MotionController.BP_MotionController_C" _returnvalue "AdjustIfPossibleButAlwaysSpawn" _self "Left" "1.000000,1.000000,1.000000" 0))
      (bind _output_get (Variables|Default|SetLeftHand _returnvalue_2))
      (Transformation|AttachComponentToComponent _output_get _vrcamroot "None" "SnapToTarget" "SnapToTarget" "KeepRelative" true))
    (:then_1
      (bind _returnvalue_3 (Game|SpawnActorfromClass "/MixedRealityFramework/Calibration/VRTemplate/Blueprints/BP_MotionController.BP_MotionController_C" _returnvalue "AdjustIfPossibleButAlwaysSpawn" _self "Right" "1.000000,1.000000,1.000000" 0))
      (bind _output_get_2 (Variables|Default|SetRightHand _returnvalue_3))
      (Transformation|AttachComponentToComponent _output_get_2 _vrcamroot "None" "SnapToTarget" "SnapToTarget" "KeepRelative" true))))

(event Collision|EventActorBeginOverlap
  (params (OtherActor :type Actor%20Object%20Reference)))

(event EventTick
  (params (DeltaSeconds :type Float%20%28single-precision%29)))

(event Input|AxisEvents|InputAxisforward
  (params (AxisValue :type Float%20%28single-precision%29))
  (Pawn|Input|AddMovementInput (Math|Vector|GetForwardVector (Math|Rotator|MakeRotator 0.0 0.0 (.yaw (Pawn|GetControlRotation :!class /Script/Engine.Pawn)))) AxisValue false))

(event Input|AxisEvents|InputAxisright
  (params (AxisValue :type Float%20%28single-precision%29))
  (Pawn|Input|AddMovementInput (Math|Vector|GetRightVector (Math|Rotator|MakeRotator 0.0 0.0 (.yaw (Pawn|GetControlRotation :!class /Script/Engine.Pawn)))) AxisValue false))

(fn ConstructionScript)