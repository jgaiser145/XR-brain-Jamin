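; bp_AmbientControler is an actor that plays four ambient audio components in a repeating, loosely timed sequence.
; On BeginPlay, a DoN gate starts Ambi1 through Ambi4 in order, with a short random delay before each.
; The gate resets after Ambi4 starts, and that component's OnAudioFinished event re-enters it to repeat the sequence with fresh delays.
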(event Custom|Playagain
  (bind _ambi4 (Variables|Default|GetAmbi4))
  (Utilities|FlowControl|DoN 1 :!label _label
    (:Exit
      (Utilities|FlowControl|Delay (Math|Random|RandomFloatinRange 0.2 2.0))
      (Audio|Components|Audio|Play (Variables|Default|Getambi1) 0.0)
      (Utilities|FlowControl|Delay (Math|Random|RandomFloatinRange 0.5 1.0))
      (Audio|Components|Audio|Play (Variables|Default|GetAmbi2) 0.0)
      (Utilities|FlowControl|Delay (Math|Random|RandomFloatinRange 0.2 1.0))
      (Audio|Components|Audio|Play (Variables|Default|GetAmbi3) 0.0)
      (Utilities|FlowControl|Delay (Math|Random|RandomFloatinRange 1.0 1.5))
      (Audio|Components|Audio|Play _ambi4 0.0)
      (EventDispatchers|BindEventtoOnAudioFinished _ambi4 (delegate Custom|Playagain))
      (goto _label Reset))))

(event EventBeginPlay
  (bind _ambi4 (Variables|Default|GetAmbi4))
  (Utilities|FlowControl|DoN 1 :!label _label
    (:Exit
      (Utilities|FlowControl|Delay (Math|Random|RandomFloatinRange 0.2 2.0))
      (Audio|Components|Audio|Play (Variables|Default|Getambi1) 0.0)
      (Utilities|FlowControl|Delay (Math|Random|RandomFloatinRange 0.5 1.0))
      (Audio|Components|Audio|Play (Variables|Default|GetAmbi2) 0.0)
      (Utilities|FlowControl|Delay (Math|Random|RandomFloatinRange 0.2 1.0))
      (Audio|Components|Audio|Play (Variables|Default|GetAmbi3) 0.0)
      (Utilities|FlowControl|Delay (Math|Random|RandomFloatinRange 1.0 1.5))
      (Audio|Components|Audio|Play _ambi4 0.0)
      (EventDispatchers|BindEventtoOnAudioFinished _ambi4 (delegate Custom|Playagain))
      (goto _label Reset))))

(event Collision|EventActorBeginOverlap
  (params (OtherActor :type Actor%20Object%20Reference)))

(event EventTick
  (params (DeltaSeconds :type Float%20%28single-precision%29)))

(fn ConstructionScript)