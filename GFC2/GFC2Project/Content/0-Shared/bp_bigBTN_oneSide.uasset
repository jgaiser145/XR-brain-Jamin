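; Shared big one-sided button actor that animates its top and plays a sound when pressed or released.
; Custom events btnPressed and btnUnpressed are guarded by an IsPressed flag, playing or reversing the BtnClicked timeline.
; The timeline drives the Top component's relative Z and calls Play on RightSound at every update, in both directions.
; The blueprint contains no trigger logic of its own.
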(event Custom|btnPressed
  (if (not (Variables|Default|GetisPressed))
    (Variables|Default|SetisPressed true)
    (bind _z_movement (Timeline|btnClicked Play)
      (:Update
        (Transformation|SetRelativeLocation (Variables|Default|GetTop) (Math|Vector|MakeVector 0.0 0.0 _z_movement) false false)
        ;[1 1 1] Noise
        (Audio|Components|Audio|Play (Variables|Default|GetRightSound) 0.0)))))

(event Custom|btnUnpressed
  (if (Variables|Default|GetisPressed)
    (Variables|Default|SetisPressed false)
    (bind _z_movement (Timeline|btnClicked Reverse)
      (:Update
        (Transformation|SetRelativeLocation (Variables|Default|GetTop) (Math|Vector|MakeVector 0.0 0.0 _z_movement) false false)
        ;[1 1 1] Noise
        (Audio|Components|Audio|Play (Variables|Default|GetRightSound) 0.0)))))

(event EventBeginPlay)

(event Collision|EventActorBeginOverlap
  (params (OtherActor :type Actor%20Object%20Reference)))

(event EventTick
  (params (DeltaSeconds :type Float%20%28single-precision%29)))

(fn ConstructionScript)